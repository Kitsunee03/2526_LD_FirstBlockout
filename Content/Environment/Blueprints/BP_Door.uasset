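; BP_Door is a hinged door that swings open when the first-person character enters its trigger and closes when they leave.
; Overlap events play and reverse a rotation timeline, whose alpha scales an Angle value into the Door component's relative yaw.
; A loose comparison of the door-to-player direction against the actor's forward vector picks the sign, so swing direction depends on the player's side.
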(event OnComponentBeginOverlap(Trigger)
  (params (OverlappedComponent :type Primitive%20Component%20Object%20Reference) (OtherActor :type Actor%20Object%20Reference) (OtherComp :type Primitive%20Component%20Object%20Reference) (OtherBodyIndex :type Integer) (bFromSweep :type Boolean) (SweepResult :type Hit%20Result%20Structure%20%28by%20ref%29))
  (bind _asbp_first_person_character (Utilities|Casting|CastToBP_FirstPersonCharacter OtherActor))
  (Variables|Default|SetDirection (Utilities|Operators|EqualEqual (Math|Vector|GetUnitDirection(Vector) (Transformation|GetActorLocation) (Transformation|GetActorLocation _asbp_first_person_character)) (Transformation|GetActorForwardVector) 1.0))
  (bind _alpha (Timeline|TL_Rotation Play)
    (:Update
      (Transformation|SetRelativeRotation (Variables|Default|GetDoor) (Math|Rotator|MakeRotator 0.0 0.0 (* _alpha (Variables|Config|GetAngle) (Math|Float|SelectFloat 1.0 -1.0 (Variables|Default|GetDirection)))) false false))))

(event OnComponentEndOverlap(Trigger)
  (params (OverlappedComponent :type Primitive%20Component%20Object%20Reference) (OtherActor :type Actor%20Object%20Reference) (OtherComp :type Primitive%20Component%20Object%20Reference) (OtherBodyIndex :type Integer))
  (Utilities|Casting|CastToBP_FirstPersonCharacter OtherActor)
  (bind _alpha (Timeline|TL_Rotation Reverse)
    (:Update
      (Transformation|SetRelativeRotation (Variables|Default|GetDoor) (Math|Rotator|MakeRotator 0.0 0.0 (* _alpha (Variables|Config|GetAngle) (Math|Float|SelectFloat 1.0 -1.0 (Variables|Default|GetDirection)))) false false))))

(fn ConstructionScript)